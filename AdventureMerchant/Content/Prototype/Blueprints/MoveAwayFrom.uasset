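; Behavior tree task for the bunny AI controller that steps its pawn away from the blackboard's ObjectToAvoid.
; It issues AIMoveTo toward a point a short fixed distance from the controller's location along that object's velocity direction.
; It then writes the point to TargetLocation and finishes successfully without waiting for the move result.
; GetAvoidanceVector is an empty, unused stub.
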(event EventReceiveExecute
  (params (OwnerActor :type Actor%20Object%20Reference))
  (bind _returnvalue (Transformation|GetActorLocation OwnerActor))
  (bind _objecttoavoid (Variables|Default|GetObjectToAvoid))
  (bind _returnvalue_2 (AI|BehaviorTree|GetBlackboardValueasActor _objecttoavoid))
  (bind _returnvalue_3 (Transformation|GetVelocity _returnvalue_2))
  (bind _returnvalue_4 (Math|Vector|Normalize _returnvalue_3))
  (bind _returnvalue_5 (* _returnvalue_4 5e+01))
  (bind _returnvalue_6 (+ _returnvalue_5 _returnvalue))
  (bind _asbunny_controller (Utilities|Casting|CastToBunnyController OwnerActor))
  (AI|AIMoveTo (Pawn|GetControlledPawn _asbunny_controller) _returnvalue_6 0 1e+01 false
    (:then
      (AI|BehaviorTree|SetBlackboardValueasVector (Variables|Default|GetTargetLocation) _returnvalue_6)
      (AI|BehaviorTree|FinishExecute true))))

(fn GetAvoidanceVector
  (params (Velocity%20to%20avoid :type Vector)))