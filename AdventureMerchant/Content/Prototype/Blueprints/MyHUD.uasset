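; MyHUD is a HUD Blueprint that draws a centered reticle while the player is in first-person view.
; On each DrawHUD it casts the player character to ThirdPersonCharacter and checks its CameraIsFirstPerson flag.
; When the flag is set, it draws the M_Cart material as a square sized by ReticleSize at the screen center.
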(event EventBeginPlay)

(event Collision|EventActorBeginOverlap
  (params (OtherActor :type Actor%20Object%20Reference)))

(event EventTick
  (params (DeltaSeconds :type Float%20%28single-precision%29)))

(event EventDrawHUD
  (params (SizeX :type Integer) (SizeY :type Integer))
  (bind _reticlesize (Variables|Default|GetReticleSize))
  (bind _returnvalue (/ _reticlesize 2.0))
  (bind _asthird_person_character (Utilities|Casting|CastToThirdPersonCharacter (Game|GetPlayerCharacter 0)))
  (if (Variables|/Game/ThirdPersonBP/Blueprints/ThirdPersonCharacter.ThirdPersonCharacter_C|GetCameraIsFirstPerson _asthird_person_character)
    (Canvas|DrawMaterial "/Game/Prototype/Materials/M_Cart.M_Cart" (- (/ (Math|Conversions|ToFloat(Integer) SizeX) 2.0) _returnvalue) (- (/ (Math|Conversions|ToFloat(Integer) SizeY) 2.0) _returnvalue) _reticlesize _reticlesize 1.0 1.0 1.0 1.0)))

(fn ConstructionScript)